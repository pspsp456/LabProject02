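; Enemy actor Blueprint with a health value that removes itself from the game when that health runs out.
; BeginPlay sets the starting HP and caches a reference to MyGameMode.
; Tick polls HP, then destroys the actor at zero or below and calls DecreaseEnemy on the game mode.
; Nothing in these graphs reduces HP, and the overlap event and construction script are empty.
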(event `self.ReceiveBeginPlay`
  (set `self.HP` 50.0)
  (bind _asmy_game_mode (cast `/Game/MyGameMode` (`GameplayStatics.GetGameMode`)))
  (set `self.GameMode` _asmy_game_mode))

(event `self.ReceiveTick`
  (params (DeltaSeconds :type "Float (single-precision)"))
  (if (<= (`self.HP`) 0.0)
    (`self.K2_DestroyActor`)
    (`/Game/MyGameMode.Decrease Enemy` (`self.GameMode`))))

(fn `UserConstructionScript`)